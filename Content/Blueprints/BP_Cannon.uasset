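; BP_Cannon is an automated turret that patrols, detects the first-person player and fires projectiles at them.
; Each tick the tower either sweeps between yaw limits or smoothly tracks the player within them, while a debug-drawn forward line trace looks for targets.
; A hit starts chasing, triggers delay-throttled shots with sound, and resets a timer meant to end the chase.
; At zero health it swaps itself for a destroyed cannon actor.
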(event Custom|Disable%20chasing
  ;[1 1 1] Rotations
  (Variables|Default|SetIsChasingPlayer? false))

(event Custom|Shoot
  (bind _trace_start_location (Variables|Default|GetTrace%20Start%20Location))
  (bind _returnvalue (Transformation|GetWorldTransform _trace_start_location))
  ;[1 1 1] Shooting
  (Utilities|FlowControl|Delay (Variables|Parameters|GetTime%20between%20shots))
  (Game|SpawnActorfromClass "/Game/Blueprints/BP_Projectile.BP_Projectile_C" (Math|Transform|MakeTransform (.location _returnvalue) (.rotation _returnvalue) "0.100000,0.100000,0.100000") "Undefined" 0 0)
  (Audio|PlaySoundatLocation "/Game/Sounds/Turret_shot.Turret_shot" (.location (Transformation|GetWorldTransform (Variables|Default|GetTrace%20Start%20Location))) "0, 0, 0" 1.0 1.0 0.0 0 0 0))

(event EventTick
  (params (DeltaSeconds :type Float%20%28single-precision%29))
  (bind _returnvalue (Utilities|Time|GetWorldDeltaSeconds))
  (bind _returnvalue_2 (Game|GetPlayerCharacter 0))
  (bind _returnvalue_3 (Transformation|GetActorTransform))
  (bind _chase_speed (Variables|Parameters|GetChase%20Speed))
  (bind _tower (Variables|Default|GetTower))
  (bind _tower_2 (Variables|Default|GetTower))
  (bind _returnvalue_4 (Transformation|GetActorLocation _returnvalue_2))
  (bind _relativerotation (Variables|/Script/Engine.SceneComponent|GetRelativeRotation _tower))
  (bind _relativelocation (Variables|/Script/Engine.SceneComponent|GetRelativeLocation _tower))
  (bind _returnvalue_5 (Math|Transform|InverseTransformLocation _returnvalue_3 _returnvalue_4))
  (bind _returnvalue_6 (Math|Rotator|FindLookatRotation _relativelocation _returnvalue_5))
  (bind _returnvalue_7 (Math|Interpolation|RInterpTo _relativerotation _returnvalue_6 _returnvalue _chase_speed))
  ;[1 1 1] Sequences
  ;[1 1 1] Check Healtpoints
  (if (<= (Variables|Default|GetHealthPoints) 0)
    ;[1 1 1] Spawn destoryed cannon
    (Game|SpawnActorfromClass "/Game/Blueprints/BP_CannonDestroyed.BP_CannonDestroyed_C" (Math|Conversions|ToTransform(Vector) (Transformation|GetWorldLocation (Variables|Default|GetDefaultSceneRoot))) "Undefined" 0 0)
    (Actor|DestroyActor)
    (elif (Variables|Default|GetIsChasingPlayer?)
      (Utilities|IsValid (Game|GetPlayerCharacter 0)
        (:Is%20Valid
          (Utilities|FlowControl|Sequence
            (:then_0
              ;[1 1 1] Rotations
              (CallFunction|TraceForward :!label _label))
            (:then_1
              (if (<= (.yaw _returnvalue_7) 0.0)
                (Transformation|SetRelativeRotation _tower_2 (Math|Rotator|MakeRotator 0.0 0.0 (Math|Float|Clamp(Float) (.yaw _returnvalue_7) (* (Math|Float|Absolute(Float) (Variables|Parameters|GetMax%20Angle)) -1.0))) false false)
                (else
                  (Transformation|SetRelativeRotation _tower_2 (Math|Rotator|MakeRotator 0.0 0.0 (Math|Float|Clamp(Float) (.yaw _returnvalue_7) 0.0 (Math|Float|Absolute(Float) (Variables|Parameters|GetMax%20Angle)))) false false)))))))
      (else
        (Utilities|FlowControl|Sequence
          (:then_0
            ;[1 1 1] Rotates the turret and reverses rotation when z(yaw) is equal to max angle
            (Transformation|AddRelativeRotation (Variables|Default|GetTower) (Math|Rotator|MakeRotator 0.0 0.0 (Variables|Parameters|GetPatrol%20Speed)) false false)
            (if (Math|Float|NearlyEqual(Float) (.Yaw (Math|Rotator|BreakRotator (Variables|/Script/Engine.SceneComponent|GetRelativeRotation (Variables|Default|GetTower)))) (Variables|Parameters|GetMax%20Angle) 1.0)
              (Variables|Parameters|SetPatrol%20Speed (* (Variables|Parameters|GetPatrol%20Speed) -1.0))
              (Variables|Parameters|SetMax%20Angle (* (Variables|Parameters|GetMax%20Angle) -1.0))))
          (:then_1
            (goto _label)))))))

(fn ConstructionScript)

(fn TraceForward
  (bind _trace_start_location (Variables|Default|GetTrace%20Start%20Location))
  (bind _returnvalue (Transformation|GetWorldLocation _trace_start_location))
  (bind _outhit (Collision|LineTraceForObjects _returnvalue (+ _returnvalue (* (Math|Vector|GetForwardVector _trace_start_location) 3e+03)) (Utilities|Array|MakeArray "ObjectTypeQuery1" "ObjectTypeQuery3") false 0 "ForOneFrame"))
  (Utilities|Casting|CastToFirstPersonCharacter (.HitActor (Collision|BreakHitResult _outhit)))
  (Variables|Default|SetIsChasingPlayer? true)
  (CallFunction|Shoot)
  (Utilities|Time|SetTimerbyFunctionName 0 "Disable Chasing" (Variables|Parameters|GetChasing%20timeout)))